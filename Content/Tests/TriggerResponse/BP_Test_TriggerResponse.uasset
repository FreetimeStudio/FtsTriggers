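; BP_Test_TriggerResponse is a functional test that checks an observed trigger reports triggered and untriggered as a character enters and leaves it.
; PrepareTest binds the trigger's message component events to a Triggered flag and spawns an AI Character at the test actor's location.
; StartTest moves the character to the trigger and back, asserting the flag after each move.
; A failed move finishes the test with an error.
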(event `self.ReceivePrepareTest`
  (bind (_returnvalue_location _returnvalue_rotation) (`KismetMathLibrary.BreakTransform` (`self.GetTransform`)))
  (bind _returnvalue (message `FtsTriggerInterface.GetTriggerComponent` (`self.ObservedTrigger`)))
  (add `FtsTriggerComponent.OnUnTriggered` _returnvalue (delegate `OnUnTriggered_Event_0`))
  (add `FtsTriggerComponent.OnTriggered` _returnvalue (delegate `OnTriggered_Event_0`))
  (bind _returnvalue_2 (`AIBlueprintHelperLibrary.SpawnAIFromClass` "/Script/Engine.Character" null _returnvalue_location _returnvalue_rotation false null))
  (set `self.TestCharacter` _returnvalue_2))

(event `OnUnTriggered_Event_0`
  (params (Trigger :type "FtsTriggerComponent Object Reference") (Instigator :type "Object Object Reference"))
  (set `self.bTriggered` false))

(event `OnTriggered_Event_0`
  (params (Trigger :type "FtsTriggerComponent Object Reference") (Instigator :type "Object Object Reference"))
  (set `self.bTriggered` true))

(event `self.ReceiveStartTest`
  (`|AIMoveTo` (`self.TestCharacter`) (0.0 0.0 0.0) (`self.ObservedTrigger`)
    (:`OnSuccess`
      (`self.AssertTrue` (`self.bTriggered`) "Overlapping Trigger")
      (`|AIMoveTo` (`self.TestCharacter`) (0.0 0.0 0.0) self
        (:`OnSuccess`
          (`self.AssertFalse` (`self.bTriggered`) "Not overlapping Trigger")
          (`self.FinishTest` "Default"))
        (:`OnFail`
          (`self.FinishTest` "Error" "Unable to move pawn" :!label _label))))
    (:`OnFail`
      (goto _label))))

(fn `UserConstructionScript`)