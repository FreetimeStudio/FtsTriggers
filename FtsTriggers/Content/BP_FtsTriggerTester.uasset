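; BP_FtsTriggerTester is a debug actor for testing the trigger system through its TriggerListener component.
; On BeginPlay it registers its Triggers array with the listener.
; When the listener reports a trigger or untrigger, it prints a message naming itself, the trigger and the instigator.
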(event `self.ReceiveBeginPlay`
  (`FtsTriggerListenerComponent.AddTriggers` (`self.TriggerListener`) (`self.Triggers`)))

(event `self.TriggerListener.OnTriggered`
  (params (Listener :type "FtsTriggerListenerComponent Object Reference") (Trigger :type "FtsTriggerComponent Object Reference") (Instigator :type "Object Object Reference"))
  (`KismetSystemLibrary.PrintText` (`|FormatText` "{Tester} got TRIGGERED by: \n{Trigger} instigatex by: \n{Instigator}" (`KismetTextLibrary.Conv_StringToText` (`KismetSystemLibrary.GetDisplayName` self)) (`KismetTextLibrary.Conv_StringToText` (`KismetSystemLibrary.GetDisplayName` Trigger)) (`KismetTextLibrary.Conv_StringToText` (`KismetSystemLibrary.GetDisplayName` Instigator)))))

(event `self.TriggerListener.OnUnTriggered`
  (params (Listener :type "FtsTriggerListenerComponent Object Reference") (Trigger :type "FtsTriggerComponent Object Reference") (Instigator :type "Object Object Reference"))
  (`KismetSystemLibrary.PrintText` (`|FormatText` "{Tester} got UN TRIGGERED by: \n{Trigger} instigatex by: \n{Instigator}" (`KismetTextLibrary.Conv_StringToText` (`KismetSystemLibrary.GetDisplayName` self)) (`KismetTextLibrary.Conv_StringToText` (`KismetSystemLibrary.GetDisplayName` Trigger)) (`KismetTextLibrary.Conv_StringToText` (`KismetSystemLibrary.GetDisplayName` Instigator)))))

(fn `UserConstructionScript`)